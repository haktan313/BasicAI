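; BP_EnemyBase is the base enemy character for a basic AI system, with functions for patrol, movement speed, attack ranges and attack tokens.
; Token requests pass through to the BPCTokens component, and movement speed maps an Idle, Walk or Jog enum to MaxWalkSpeed.
; EnemyAttack switches on melee, range or explosion but only prints placeholders for child classes, and SetRange returns zero attack and defense radii.
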(event `/Game/HaktanThing_BasicAISystem/BPI_Tokens.giveTokenToTarget`
  (params (AmountOfToken :type Integer))
  (`/Game/HaktanThing_BasicAISystem/BPC_Tokens.giveTokenToTarget` (`self.BPC_Tokens`) AmountOfToken))

(event `/Game/HaktanThing_BasicAISystem/AI/BPI_AISystem.enemyAttack`
  (params (enemyAttackType :type "/Game/HaktanThing_BasicAISystem/AI/Enum/E_AttackType Enum" :default "NewEnumerator0"))
  (switch `/Game/HaktanThing_BasicAISystem/AI/Enum/E_AttackType` enemyAttackType
    (:`NewEnumerator0`
      (`KismetSystemLibrary.PrintString` "addMeleeChildObject"))
    (:`NewEnumerator1`
      (`KismetSystemLibrary.PrintString` "addRangeChildObject"))
    (:`NewEnumerator2`
      (`KismetSystemLibrary.PrintString` "addExplosiveChildObject"))))

(fn `Patrol`
  (returns (patrol :type "/Game/HaktanThing_BasicAISystem/AI/BP_Patrol Object Reference"))
  (return (`self.patroObject`)))

(fn `setMovementSpeed`
  (params (movementSpeedEnum :type "/Game/HaktanThing_BasicAISystem/AI/Enum/E_MovementSpeed Enum" :default "NewEnumerator0"))
  (returns (newSpeed :type "Float (double-precision)"))
  (bind _output_get (set `CharacterMovementComponent.MaxWalkSpeed` (select `/Game/HaktanThing_BasicAISystem/AI/Enum/E_MovementSpeed` movementSpeedEnum :`NewEnumerator1` 300.0 :`NewEnumerator2` 600.0 :!type "Float (single-precision)") (`self.CharacterMovement`)))
  (return _output_get))

(fn `setRange`
  (returns (Radius :type "/Game/HaktanThing_BasicAISystem/AI/S_Range Structure"))
  (return (make `/Game/HaktanThing_BasicAISystem/AI/S_Range` 0.0)))

(fn `tookTokenForAttack`
  (params (AmountOfToken :type Integer))
  (returns (Success :type Boolean))
  (bind _success (`/Game/HaktanThing_BasicAISystem/BPC_Tokens.tookTokenForAttack` (`self.BPC_Tokens`) AmountOfToken))
  (return _success))

(fn `UserConstructionScript`)