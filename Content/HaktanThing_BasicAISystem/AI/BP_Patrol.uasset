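; BP_Patrol is a spline-based patrol route for the basic AI system.
; PatrolRouteIndexAdjust steps the current point index by a direction value, ping-ponging by flipping direction at either limit.
; The upper limit is tested as the spline point count minus negative one, so it sits past the last valid index.
; SplineWorldLocation returns the world position of the current spline point.
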(event `PatrolRouteIndexAdjust`
  (bind _output_get (set `self.currentPointIndex` (+ (`self.currentPointIndex`) (`self.direction`))))
  (if (== _output_get (- (`SplineComponent.GetNumberOfSplinePoints` (`self.Spline`)) -1))
    (set `self.direction` -1)
    (elif (== (`self.currentPointIndex`) 0)
      (set `self.direction` 1))))

(fn `splineWorldLocation`
  (returns (worldPosition :type "Vector Structure"))
  (return (`SplineComponent.GetLocationAtSplinePoint` (`self.Spline`) (`self.currentPointIndex`) "World")))

(fn `UserConstructionScript`)