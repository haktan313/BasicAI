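; AI controller for enemies derived from BP_EnemyBase, switching them between Idle, Investigate and Attack states.
; On possess it runs the pawn's behavior tree, sets Idle and writes attack and defense radii to the Blackboard.
; Perception updates for Player-tagged actors check sight, hearing and damage separately.
; While idle or investigating, noise triggers Investigate, damage triggers Attack, and sight triggers Attack only for the existing Blackboard target.
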(event `self.ReceivePossess`
  (params (PossessedPawn :type "Pawn Object Reference"))
  (bind _asbp_enemy_base (cast `/Game/HaktanThing_BasicAISystem/BP_EnemyBase` PossessedPawn))
  (bind _output_get (set `self.As BP Enemy Base` _asbp_enemy_base))
  (`self.RunBehaviorTree` (`/Game/HaktanThing_BasicAISystem/BP_EnemyBase.behaviorTree` _output_get))
  (`self.setStateIdle`)
  (bind _radius (message `/Game/HaktanThing_BasicAISystem/AI/BPI_AISystem.setRange` (`self.As BP Enemy Base`)))
  (`BlackboardComponent.SetValueAsFloat` (`self.Blackboard`) (`self.attackRadius`) (break `/Game/HaktanThing_BasicAISystem/AI/S_Range` _radius))
  (`BlackboardComponent.SetValueAsFloat` (`self.Blackboard`) (`self.defanceRadius`) (`.DefanceRadius_4_1B8E3C994923FE6B5FD2E0BA1EDA9EDD` (break `/Game/HaktanThing_BasicAISystem/AI/S_Range` _radius))))

(event `self.AIPerception.OnPerceptionUpdated`
  (params (UpdatedActors :type "Array of Actor Object Reference (by ref)"))
  (for _array_element UpdatedActors
    (if (`self.ActorHasTag` _array_element "Player")
      (set `self.SensedActor` _array_element)
      (`|ExecutionSequence`
        (:`then_0`
          (bind _successfully_sensed (`self.CanSenseActor?` (`self.SensedActor`)))
          (if _successfully_sensed
            (`self.SeeReaction` (`self.SensedActor`))))
        (:`then_1`
          (bind (_successfully_sensed_2 _array_element_2) (`self.CanSenseActor?` (`self.SensedActor`) "NewEnumerator1"))
          (if _successfully_sensed_2
            (`self.HearReaction` (`.StimulusLocation` (break `AIStimulus` _array_element_2)))))
        (:`then_2`
          (bind _successfully_sensed_3 (`self.CanSenseActor?` (`self.SensedActor`) "NewEnumerator2"))
          (if _successfully_sensed_3
            (`self.damageReaction` (`self.SensedActor`))))))))

(fn `CanSenseActor?`
  (params (Actor :type "Actor Object Reference") (Sense :type "/Game/HaktanThing_BasicAISystem/AI/Enum/E_SenseType Enum" :default "NewEnumerator0"))
  (returns (`Successfully Sensed` :type Boolean) (`Array Element` :type "AIStimulus Structure"))
  (bind _info (`AIPerceptionComponent.GetActorsPerception` (`self.AIPerception`) Actor))
  (for _array_element (`.LastSensedStimuli` (break `ActorPerceptionBlueprintInfo` _info))
    (bind _returnvalue (`AIPerceptionSystem.GetSenseClassForStimulus` _array_element))
    (if (== _returnvalue (select `/Game/HaktanThing_BasicAISystem/AI/Enum/E_SenseType` Sense :`NewEnumerator0` "/Script/AIModule.AISense_Sight" :`NewEnumerator1` "/Script/AIModule.AISense_Hearing" :`NewEnumerator2` "/Script/AIModule.AISense_Damage" :!type "Object Class Reference"))
      (return (`.bSuccessfullySensed` (break `AIStimulus` _array_element)) _array_element))))

(fn `damageReaction`
  (params (Actor :type "Actor Object Reference"))
  (bind _state (`self.GetCurrentState`))
  (switch `/Game/HaktanThing_BasicAISystem/AI/Enum/E_StateType` _state
    (:`NewEnumerator0`
      _)
    (:`NewEnumerator1`
      _))
  (`self.setStateAttack` Actor))

(fn `GetCurrentState`
  (returns (State :type "/Game/HaktanThing_BasicAISystem/AI/Enum/E_StateType Enum"))
  (return (cast `/Game/HaktanThing_BasicAISystem/AI/Enum/E_StateType` (`BlackboardComponent.GetValueAsEnum` (`self.Blackboard`) (`self.stateKeyName`)))))

(fn `HearReaction`
  (params (Vector :type "Vector Structure"))
  (bind _state (`self.GetCurrentState`))
  (switch `/Game/HaktanThing_BasicAISystem/AI/Enum/E_StateType` _state
    (:`NewEnumerator0`
      _)
    (:`NewEnumerator1`
      _))
  (`self.setStateInvestigate` Vector))

(fn `SeeReaction`
  (params (Actor :type "Actor Object Reference"))
  (bind _state (`self.GetCurrentState`))
  (switch `/Game/HaktanThing_BasicAISystem/AI/Enum/E_StateType` _state
    (:`NewEnumerator0`
      _)
    (:`NewEnumerator1`
      _))
  (if (== Actor (`BlackboardComponent.GetValueAsObject` (`self.Blackboard`) (`self.targetActorKeyName`)))
    (`self.setStateAttack` Actor)))

(fn `setStateAttack`
  (params (Actor :type "Actor Object Reference"))
  (`BlackboardComponent.SetValueAsObject` (`self.Blackboard`) (`self.targetActorKeyName`) Actor)
  (`BlackboardComponent.SetValueAsEnum` (`self.Blackboard`) (`self.stateKeyName`) (enumliteral `/Game/HaktanThing_BasicAISystem/AI/Enum/E_StateType` "NewEnumerator2")))

(fn `setStateIdle`
  (`BlackboardComponent.SetValueAsEnum` (`self.Blackboard`) (`self.stateKeyName`) (enumliteral `/Game/HaktanThing_BasicAISystem/AI/Enum/E_StateType` "NewEnumerator0")))

(fn `setStateInvestigate`
  (params (Vector :type "Vector Structure"))
  (`BlackboardComponent.SetValueAsVector` (`self.Blackboard`) (`self.pointOfInterest`) Vector)
  (`BlackboardComponent.SetValueAsEnum` (`self.Blackboard`) (`self.stateKeyName`) (enumliteral `/Game/HaktanThing_BasicAISystem/AI/Enum/E_StateType` "NewEnumerator1")))

(fn `UserConstructionScript`)