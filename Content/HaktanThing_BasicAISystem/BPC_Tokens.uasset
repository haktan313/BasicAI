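; BPC_Tokens is a component in the basic AI system that holds an attack token pool.
; TookTokenForAttack subtracts the requested amount from the current count and returns true when enough tokens remain, otherwise it returns false.
; GiveTokenToTarget adds tokens back to the count, with no upper limit check.
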(fn `giveTokenToTarget`
  (params (AmountOfToken :type Integer))
  (set `self.currentToken` (+ (`self.currentToken`) AmountOfToken)))

(fn `tookTokenForAttack`
  (params (AmountOfToken :type Integer))
  (returns (Success :type Boolean))
  (if (>= (`self.currentToken`) AmountOfToken)
    (set `self.currentToken` (- (`self.currentToken`) AmountOfToken))
    (return true)
    (else
      (return false))))